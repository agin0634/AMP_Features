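; Trail actor that follows one tracked point, by ID, from the BP_URGSeries DBSCAN aggregator, drawing a spline with a particle system along it.
; Point-move events and a per-Tick search of aggregated points append spline points past a spawn distance and reposition the particles.
; A gate toggled by draw start/end events also runs appending plus neighbor-average smoothing on Tick.
; DestroySelf removes the actor after a delay.
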(event Custom|DrawSplineStart
  (params (Location :type Vector))
  (Utilities|FlowControl|Gate true) ; enters at Open
)

(event Custom|DrawSplineEnd
  (Utilities|FlowControl|Gate true) ; enters at Close
)

(event Custom|DestroySelf
  (Utilities|FlowControl|Delay 1e+01)
  (Actor|DestroyActor))

(event Custom|CustomEvent_0
  (params (Point :type Aggregated%20Point%20Structure%20%28by%20ref%29) (From :type Aggregated%20Point%20Structure%20%28by%20ref%29))
  (if (== (.index Point) (Variables|Default|GetPointId))
    (CallFunction|SpawnSplinePoints (.worldlocation Point))
    (Transformation|SetWorldLocation (Variables|Default|GetParticleSystem) (Spline|GetLocationatSplinePoint (Variables|Default|GetSpline) (Variables|Default|GetPointIndex) "World") false false)))

(event Custom|URGSetSpawnPointId
  (params (PointIndex :type Integer))
  (Variables|Default|SetPointId PointIndex))

(event EventBeginPlay
  (bind _outactors (Actor|GetAllActorsOfClass "/Game/URG/BP_URGSeries.BP_URGSeries_C"))
  (bind _output_get (Variables|Default|SetCurrentURGSeries (Utilities|Array|Get(acopy) _outactors)))
  (EventDispatchers|BindEventtoOnPointMove (Variables|/Game/URG/BP_URGSeries.BP_URGSeries_C|GetAggregateDBSCAN _output_get) (delegate Custom|CustomEvent_0)))

(event EventTick
  (params (DeltaSeconds :type Float%20%28single-precision%29))
  (Utilities|FlowControl|Sequence
    (:then_0
      (Utilities|FlowControl|Gate true
        (:Exit
          (CallFunction|SpawnSplinePoints (stale Custom|DrawSplineStart Location))
          (CallFunction|SmoothSplinePoints)
          (Transformation|SetWorldLocation (Variables|Default|GetParticleSystem) (Spline|GetLocationatSplinePoint (Variables|Default|GetSpline) (Variables|Default|GetPointIndex) "World") false false))))
    (:then_1
      (bind _returnvalue (Class|URGAggregater|GetAggregatedPoints (Variables|/Game/URG/BP_URGSeries.BP_URGSeries_C|GetAggregateDBSCAN (Variables|Default|GetCurrentURGSeries))))
      (bind _array_element (Utilities|Array|ForEachLoopwithBreak _returnvalue :!label _label)
        (:LoopBody
          (if (== (.index _array_element) (Variables|Default|GetPointId))
            (CallFunction|SpawnSplinePoints (.worldlocation _array_element))
            (Transformation|SetWorldLocation (Variables|Default|GetParticleSystem) (Spline|GetLocationatSplinePoint (Variables|Default|GetSpline) (Variables|Default|GetPointIndex) "World") false false)
            (goto _label Break)))))))

(fn ConstructionScript)

(fn SpawnSplinePoints
  (params (Location :type Vector))
  (Variables|Default|SetCurrentPointLocation Location)
  (if (> (Math|Vector|VectorLength (- (Variables|Default|GetCurrentPointLocation) (Variables|Default|GetPreviousPointLocation))) (Variables|Default|GetSpawnDistance))
    (Spline|AddSplinePointatIndex (Variables|Default|GetSpline) (Variables|Default|GetCurrentPointLocation) (Variables|Default|GetPointIndex) "World" true)
    (bind _result (Math|Integer|IncrementInt (Variables|Default|GetPointIndex))
      (:%20%20
        (Variables|Default|SetPointIndex _result))))
  (Variables|Default|SetPreviousPointLocation (Variables|Default|GetCurrentPointLocation)))

(fn SmoothSplinePoints
  (if (> (Spline|GetNumberOfSplinePoints (Variables|Default|GetSpline)) 2)
    (Spline|SetLocationatSplinePoint (Variables|Default|GetSpline) (- (Variables|Default|GetPointIndex) 1) (/ (+ (Spline|GetLocationatSplinePoint (Variables|Default|GetSpline) (Variables|Default|GetPointIndex) "World") (Spline|GetLocationatSplinePoint (Variables|Default|GetSpline) (- (Variables|Default|GetPointIndex) 2) "World")) 2.0) "World" true)))