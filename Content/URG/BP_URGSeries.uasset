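; BP_URGSeries is an actor that turns clustered URG scan points into spline trail actors.
; It feeds URGDataFilter into AggregateDBSCAN as the scan data provider, then listens for that component's point enter and leave events.
; Each entering point spawns a BP_SplineTrail tagged with its index, and leaving destroys and unlists the trail with that index.
; The point-move debug binding is left unconnected.
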(event Custom|CustomEvent_2
  (params (Point :type Aggregated%20Point%20Structure%20%28by%20ref%29))
  (CallFunction|DrawSplineStart (.worldlocation Point) (.size Point) (.index Point)))

(event Custom|CustomEvent_0
  (params (Point :type Aggregated%20Point%20Structure%20%28by%20ref%29))
  (CallFunction|DrawSplindEnd (.index Point)))

(event Custom|CustomEvent_1
  (params (Point :type Aggregated%20Point%20Structure%20%28by%20ref%29) (From :type Aggregated%20Point%20Structure%20%28by%20ref%29))
  (Rendering|Debug|DrawDebugPoint (.worldlocation Point) 15.0 "(R=0.015757,G=0.000000,B=1.000000,A=1.000000)" 1e+01))

(event EventBeginPlay
  (bind _aggregatedbscan (Variables|Default|GetAggregateDBSCAN))
  (Class|URGAggregater|SetScanDataProvider _aggregatedbscan (Variables|Default|GetURGDataFilter))
  (EventDispatchers|BindEventtoOnPointEnter _aggregatedbscan (delegate Custom|CustomEvent_2))
  (EventDispatchers|BindEventtoOnPointLeave _aggregatedbscan (delegate Custom|CustomEvent_0)))

(event Collision|EventActorBeginOverlap
  (params (OtherActor :type Actor%20Object%20Reference)))

(event EventTick
  (params (DeltaSeconds :type Float%20%28single-precision%29)))

(fn ConstructionScript
  (Class|URGAggregater|SetScanDataProvider (Variables|Default|GetAggregateDBSCAN) (Variables|Default|GetURGDataFilter)))

(fn DrawSplineStart
  (params (Location :type Vector) (Size :type Integer) (Index :type Integer))
  (LocalVariables|SetPointLocation Location)
  (LocalVariables|SetPointSize Size)
  (LocalVariables|SetPointIndex Index)
  (bind _returnvalue (Game|SpawnActorfromClass "/Game/AMP/Blueprint/BP_SplineTrail.BP_SplineTrail_C" (Math|Transform|MakeTransform (LocalVariables|GetPointLocation) "0, 0, 0" "3.000000,3.000000,3.000000") "Undefined" 0 0))
  (Default|URGSetSpawnPointId _returnvalue (LocalVariables|GetPointIndex))
  (Utilities|Array|Add (Variables|Default|GetSTs) _returnvalue))

(fn DrawSplindEnd
  (params (Index :type Integer))
  (LocalVariables|SetPointIndex Index)
  (bind _array_element (Utilities|Array|ForEachLoopwithBreak (Variables|Default|GetSTs) :!label _label)
    (:LoopBody
      (if (== (Variables|/Game/AMP/Blueprint/BP_SplineTrail.BP_SplineTrail_C|GetPointId _array_element) (LocalVariables|GetPointIndex))
        (Default|DestroySelf _array_element)
        (Utilities|Array|RemoveItem (Variables|Default|GetSTs) _array_element)
        (goto _label Break)))))