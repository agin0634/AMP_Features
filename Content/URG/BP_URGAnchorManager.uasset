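; BP_URGAnchorManager connects URG sensors and runs searches that match them to anchors by index.
; On BeginPlay it connects all URGs and binds handlers for found-URG and finding-score-change callbacks.
; Scan starts a search for the anchor at LocatingIndex, each find advances that index, and Stop ends the search.
; Score changes print the highest score as debug output.
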(event Custom|Scan
  (Class|URGAnchorManager|StarttoFindURGforAnchorIndex (Variables|Default|GetLocatingIndex)))

(event Custom|Stop
  (Class|URGAnchorManager|StopFindingURG))

(event Custom|CustomEvent_0
  (params (Anchor :type Actor%20Object%20Reference) (URG :type URG%20Connector%20Object%20Reference))
  (Math|Integer|IncrementInt (Variables|Default|GetLocatingIndex)))

(event Custom|CustomEvent_1
  (params (Anchor :type Actor%20Object%20Reference) (HighestScore :type Float%20%28single-precision%29))
  (Development|PrintString (Utilities|String|ToString(Float) HighestScore)))

(event EventBeginPlay
  (Class|URGAnchorManager|ConnectAllURGs)
  (EventDispatchers|BindEventtoOnFoundURG (delegate Custom|CustomEvent_0))
  (EventDispatchers|BindEventtoOnFindingScoreChange (delegate Custom|CustomEvent_1)))

(event Collision|EventActorBeginOverlap
  (params (OtherActor :type Actor%20Object%20Reference)))

(event EventTick
  (params (DeltaSeconds :type Float%20%28single-precision%29)))

(fn ConstructionScript)